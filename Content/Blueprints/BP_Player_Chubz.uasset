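; Player pawn Chubz for a shooter on the X/Z plane, with a spinning spawn animation that enables firing when finished.
; Interpolated axis input drives swept movement and mesh turning, while box hits bounce the speed off the surface.
; Looping timers repeat twin primary and secondary shots and a charge-gated ultimate, whose charge-up logic is left unconnected.
; Damage shakes the camera through the game mode, and death adds explosion effects and triggers game over.
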(event OnComponentHit(Box)
  (params (HitComponent :type Primitive%20Component%20Object%20Reference) (OtherActor :type Actor%20Object%20Reference) (OtherComp :type Primitive%20Component%20Object%20Reference) (NormalImpulse :type Vector :default "0, 0, 0") (Hit :type Hit%20Result%20Structure%20%28by%20ref%29))
  (bind (_x _y _z) (Math|Vector|BreakVector (.normal Hit)))
  (Variables|Default|SetHSpeed (* (* (Math|Float|Absolute(Float) (Variables|Default|GetHSpeed)) 2.0) _x))
  (Variables|Default|SetVSpeed (* (* (Math|Float|Absolute(Float) (Variables|Default|GetVSpeed)) 2.0) _z)))

(event Custom|PrimFire
  ;[1 1 1] Action and Movement mapping
  (CallFunction|PrimaryFire (Transformation|GetWorldTransform (Variables|Default|GetProjectileSPawnRL)))
  (CallFunction|PrimaryFire (Transformation|GetWorldTransform (Variables|Default|GetProjectileSPawnR))))

(event Custom|SeconFire
  ;[1 1 1] Action and Movement mapping
  (CallFunction|SecondryFire (Transformation|GetWorldTransform (Variables|Default|GetProjectileSPawnRL)))
  (CallFunction|SecondryFire (Transformation|GetWorldTransform (Variables|Default|GetProjectileSPawnR))))

(event Custom|UltFire
  ;[1 1 1] Action and Movement mapping
  (CallFunction|UltimateFire (Transformation|GetWorldTransform (Variables|Default|GetProjectileSPawn))))

(event EventBeginPlay
  ;[1 1 1] Spawn and Spawn Animation
  (bind _asbp_gamemode (Utilities|Casting|CastToBP_Gamemode (Game|GetGameMode)))
  (Variables|Default|SetBP_Gamemode _asbp_gamemode)
  (Variables|Default|SetYaw (.Yaw (Math|Rotator|BreakRotator (Transformation|GetActorRotation))))
  (Variables|Default|SetSpawnLocation (Transformation|GetActorLocation))
  (bind _speed (Timeline|SpawnAnimation Play)
    (:Update
      (Transformation|SetActorLocation (Math|Vector|Lerp(Vector) (Variables|Default|GetSpawnLocation) (+ (Variables|Default|GetSpawnLocation) "0, 0, 0") _speed) false false)
      (Transformation|SetRelativeRotation (Variables|Default|GetPlayerMesh) (Math|Rotator|Lerp(Rotator) "0, 0, 0" (Math|Rotator|MakeRotator 0.0 0.0 (+ (Variables|Default|GetYaw) 1.44e+03)) _speed) false false))
    (:Finished
      (Variables|Default|SetMoveEnabled true))))

(event Game|Damage|EventAnyDamage
  (params (Damage :type Float%20%28single-precision%29) (DamageType :type Damage%20Type%20Object%20Reference) (InstigatedBy :type Controller%20Object%20Reference) (DamageCauser :type Actor%20Object%20Reference))
  (bind _returnvalue (Transformation|GetActorLocation))
  (bind _returnvalue_2 (Transformation|GetActorLocation))
  (bind _bp_gamemode (Variables|Default|GetBP_Gamemode))
  (Variables|Default|SetHealth (Math|Float|Clamp(Float) (- (Variables|Default|GetHealth) Damage) 0.0 (Variables|Default|GetMaxHealth)))
  (Default|PlayCameraShake (Variables|Default|GetBP_Gamemode) "/Game/Blueprints/BP_CameraShakeSmall.BP_CameraShakeSmall_C" _returnvalue_2)
  (if (<= (Variables|Default|GetHealth) 0.0)
    (Effects|SpawnEmitteratLocation "/Game/Assets/Particles/P_Pixel_Explosion_Player.P_Pixel_Explosion_Player" _returnvalue_2)
    (Audio|PlaySoundatLocation 0 _returnvalue "0, 0, 0" 1.0 1.0 0.0 0 0 0)
    (Default|PlayCameraShake _bp_gamemode "/Game/Blueprints/BP_CameraShake.BP_CameraShake_C" _returnvalue)
    (Default|GameOver _bp_gamemode)
    (Actor|DestroyActor)))

(event EventTick
  (params (DeltaSeconds :type Float%20%28single-precision%29))
  (bind _playermesh (Variables|Default|GetPlayerMesh))
  ;[1 1 1] Comment
  (Variables|Default|SetDeltaSeconds DeltaSeconds)
  (Transformation|SetActorLocation (+ (Transformation|GetActorLocation) (Math|Vector|MakeVector (Variables|Default|GetHSpeed) 0.0 (Variables|Default|GetVSpeed))) true false)
  (Transformation|SetActorLocation (+ (Transformation|GetActorLocation) (Math|Vector|MakeVector 0.0 0.0 (Variables|Default|GetVSpeed))) true false)
  (Transformation|SetActorLocation (+ (Transformation|GetActorLocation) (Math|Vector|MakeVector (Variables|Default|GetHSpeed) 0.0 0.0)) true false)
  (Utilities|IsValid self
    (:Is%20Valid
      (Transformation|SetRelativeRotation _playermesh (Class|KismetMathLibrary|RInterptoConstant (Variables|/Script/Engine.SceneComponent|GetRelativeRotation _playermesh) (Math|Rotator|MakeRotator 0.0 0.0 (+ (* (Variables|Default|GetHSpeed) -7.0) (Variables|Default|GetYaw))) (Variables|Default|GetDeltaSeconds) 5e+01) false false))))

(event Input|ActionEvents|InputActionPrimaryFire
  (params (Key :type Key%20Structure :default "None"))
  ;[1 1 1] Action and Movement mapping
  (:Pressed
    (if (Variables|Default|GetMoveEnabled)
      (Utilities|Time|SetTimerbyFunctionName 0 "PrimFire" 0.2 true)
      (CallFunction|PrimaryFire (Transformation|GetWorldTransform (Variables|Default|GetProjectileSPawnRL)))
      (CallFunction|PrimaryFire (Transformation|GetWorldTransform (Variables|Default|GetProjectileSPawnR)))))
  (:Released
    (Utilities|Time|ClearTimerbyFunctionName 0 "PrimFire")))

(event Input|ActionEvents|InputActionSecondryFire
  (params (Key :type Key%20Structure :default "None"))
  ;[1 1 1] Action and Movement mapping
  (:Pressed
    (if (Variables|Default|GetMoveEnabled)
      (Utilities|Time|SetTimerbyFunctionName 0 "SeconFire" 0.6 true)
      (CallFunction|SecondryFire (Transformation|GetWorldTransform (Variables|Default|GetProjectileSPawnRL)))
      (CallFunction|SecondryFire (Transformation|GetWorldTransform (Variables|Default|GetProjectileSPawnR)))))
  (:Released
    (Utilities|Time|ClearTimerbyFunctionName 0 "SeconFire")))

(event Input|ActionEvents|InputActionUltimateFire
  (params (Key :type Key%20Structure :default "None"))
  ;[1 1 1] Action and Movement mapping
  (:Pressed
    (if (>= (Variables|Default|GetcurrentCharge) (Variables|Default|GetmaxCharge))
      (Utilities|Time|SetTimerbyFunctionName 0 "UltFire" 5.0)
      (if (Variables|Default|GetMoveEnabled)
        (Utilities|Time|SetTimerbyFunctionName 0 "UltFire" 0.01 true)
        (CallFunction|UltimateFire (Transformation|GetWorldTransform (Variables|Default|GetProjectileSPawn))))))
  (:Released
    (Utilities|Time|ClearTimerbyFunctionName 0 "UltFire")))

(event Input|AxisEvents|InputAxisMoveUp
  (params (AxisValue :type Float%20%28single-precision%29))
  ;[1 1 1] Action and Movement mapping
  (Variables|Default|SetVSpeed (Math|Interpolation|FInterpTo (Variables|Default|GetVSpeed) (* AxisValue (Variables|Default|GetMovementSpeed)) (Variables|Default|GetDeltaSeconds) 6.0)))

(event Input|AxisEvents|InputAxisMoveRight
  (params (AxisValue :type Float%20%28single-precision%29))
  ;[1 1 1] Action and Movement mapping
  (Variables|Default|SetHSpeed (Math|Interpolation|FInterpTo (Variables|Default|GetHSpeed) (* AxisValue (Variables|Default|GetMovementSpeed)) (Variables|Default|GetDeltaSeconds) 6.0)))

(fn ConstructionScript
  (Variables|Default|SetHealth (Variables|Default|GetMaxHealth)))

(fn PrimaryFire
  (params (SpawnTransform :type Transform))
  (Game|SpawnActorfromClass "/Game/Blueprints/Projectiles/BP_Projectile_PlayerPrimary.BP_Projectile_PlayerPrimary_C" SpawnTransform "AlwaysSpawn" 0 (LocalVariables|GetProjectile%20Color) self))

(fn SecondryFire
  (params (Spawn :type Transform))
  (Game|SpawnActorfromClass "/Game/Blueprints/Projectiles/BP_Projectile_PlayersSecondry.BP_Projectile_PlayersSecondry_C" Spawn "AlwaysSpawn" 0 (LocalVariables|GetColor) 0))

(fn UltimateFire
  (params (Spawn :type Transform))
  (Game|SpawnActorfromClass "/Game/Blueprints/Projectiles/BP_Projectile_PlayerBase.BP_Projectile_PlayerBase_C" Spawn "AlwaysSpawn" 0 (LocalVariables|GetProjectileColor) self))