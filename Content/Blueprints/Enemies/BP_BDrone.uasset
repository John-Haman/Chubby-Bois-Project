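; BP_BDrone is an enemy drone that fires projectile volleys, with a sound, based on a check against the player pawn.
; Each Tick compares DistanceFromPlayer with the absolute Z of the summed player and drone locations, rather than their difference.
; When DistanceFromPlayer is not greater, FireVolleys spawns a tinted VolleyType at four left and right mount points.
; The graph itself applies no cooldown between volleys.
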(event EventBeginPlay
  (|CallParentFunction) ; This node is disabled and will not be called.\nDrag off pins to build functionality.
)

(event Collision|EventActorBeginOverlap
  (params (OtherActor :type Actor%20Object%20Reference))
  (|CallParentFunction OtherActor) ; This node is disabled and will not be called.\nDrag off pins to build functionality.
)

(event EventTick
  (params (DeltaSeconds :type Float%20%28single-precision%29))
  (|CollapseGraph_0)
  (|CallParentFunction DeltaSeconds))

(fn ConstructionScript
  (|CallParentFunction))

(fn FireVolleys
  (bind _volleytype (Variables|Default|GetVolleyType))
  (Game|SpawnActorfromClass _volleytype (Transformation|GetWorldTransform (Variables|Default|GetLeft1)) "AlwaysSpawn" 0 "(R=0.135417,G=0.094095,B=0.004444,A=1.000000)" 0)
  (Game|SpawnActorfromClass _volleytype (Transformation|GetWorldTransform (Variables|Default|GetLeft2)) "AlwaysSpawn" 0 "(R=0.135417,G=0.094095,B=0.004444,A=1.000000)" 0)
  (Game|SpawnActorfromClass _volleytype (Transformation|GetWorldTransform (Variables|Default|GetRight1)) "AlwaysSpawn" 0 "(R=0.135417,G=0.094095,B=0.004444,A=1.000000)" 0)
  (Game|SpawnActorfromClass _volleytype (Transformation|GetWorldTransform (Variables|Default|GetRight2)) "AlwaysSpawn" 0 "(R=0.135417,G=0.094095,B=0.004444,A=1.000000)" 0))