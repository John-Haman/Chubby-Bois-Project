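; Asteroid enemy that gets a random speed and non-uniform scale and awards score when killed.
; BeginPlay caches BP_Gamemode, then feeds the random values into its projectile movement and mesh.
; EnemyKilled spawns an explosion, passes score and camera shake to the game mode, plays a sound and destroys the actor.
; Tick sets relative yaw to SpinSpeed times delta time, without accumulating rotation.
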(event EventBeginPlay
  (bind _maxscale (Variables|Default|GetMaxScale))
  (bind _projectilemovement (Variables|Default|GetProjectileMovement))
  (bind _minscale (Variables|Default|GetMinScale))
  (bind _returnvalue (Math|Random|RandomFloatinRange _minscale _maxscale))
  (bind _asbp_gamemode (Utilities|Casting|CastToBP_Gamemode (Game|GetGameMode)))
  (Variables|Default|SetBPGameMode _asbp_gamemode)
  (bind _output_get (Variables|Default|SetMoveSpeed (Math|Random|RandomFloatinRange (Variables|Default|GetMinSpeed) (Variables|Default|GetMaxSpeed))))
  (bind _output_get_2 (Variables|/Script/Engine.ProjectileMovementComponent|SetMaxSpeed _projectilemovement _output_get))
  (Variables|/Script/Engine.ProjectileMovementComponent|SetInitialSpeed _projectilemovement _output_get_2)
  (bind _output_get_3 (Variables|Default|SetScale (Math|Vector|MakeVector _returnvalue _returnvalue _returnvalue)))
  (Transformation|SetWorldScale3D (Variables|Default|GetStaticMesh) _output_get_3))

(event EventTick
  (params (DeltaSeconds :type Float%20%28single-precision%29))
  (Transformation|SetRelativeRotation (Variables|Default|GetStaticMesh) (* (Math|Rotator|MakeRotator 0.0 0.0 (Variables|Default|GetSpinSpeed)) DeltaSeconds) false false))

(event EventEnemyKilled
  (params (Location :type Vector :default "0, 0, 0"))
  (bind _returnvalue (Transformation|GetActorLocation))
  (bind _bpgamemode (Variables|Default|GetBPGameMode))
  ;[1 1 1] death
  (Effects|SpawnEmitteratLocation "/Game/Assets/Particles/P_Pixel_Explosion_Player.P_Pixel_Explosion_Player" Location "0, 0, 0" "3.000000,3.000000,3.000000")
  (Default|SetScore _bpgamemode (Variables|Default|GetEnemyScoreValue))
  (Default|PlayCameraShake _bpgamemode "/Game/Blueprints/BP_CameraShake.BP_CameraShake_C" _returnvalue)
  (Audio|PlaySoundatLocation 0 _returnvalue "0, 0, 0" 1.0 1.0 0.0 0 0 0)
  (Actor|DestroyActor))

(fn ConstructionScript
  (|CallParentFunction)
  (Transformation|SetWorldScale3D (Variables|Default|GetStaticMesh) (Variables|Default|GetScale)))