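; Base projectile for enemy attacks, with configurable color, scale, speed and damage.
; The construction script creates a dynamic material on the mesh and applies scale and speed to the mesh and projectile movement; BeginPlay sets the material color.
; On any mesh overlap it destroys itself, applying damage first only if the other actor is the player, BP_Player_Chubz.
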(event OnComponentBeginOverlap(StaticMesh)
  (params (OverlappedComponent :type Primitive%20Component%20Object%20Reference) (OtherActor :type Actor%20Object%20Reference) (OtherComp :type Primitive%20Component%20Object%20Reference) (OtherBodyIndex :type Integer) (bFromSweep :type Boolean) (SweepResult :type Hit%20Result%20Structure%20%28by%20ref%29))
  (Utilities|Casting|CastToBP_Player_Chubz OtherActor
    (:then
      (Game|Damage|ApplyDamage OtherActor (Variables|Default|GetDamage) 0 0)
      (Actor|DestroyActor))
    (:CastFailed
      (Actor|DestroyActor))))

(event EventBeginPlay
  (Rendering|Material|SetVectorParameterValue (Variables|Default|GetProjectile%20Material) "Color" (Variables|Default|GetProjcetile%20Color) :!class /Script/Engine.MaterialInstanceDynamic))

(fn ConstructionScript
  (bind _projectilemovement (Variables|Default|GetProjectileMovement))
  (bind _speed (Variables|Default|GetSpeed))
  (bind _returnvalue (Rendering|Material|CreateDynamicMaterialInstance (Variables|Default|GetStaticMesh) 0 0 "None" :!class /Script/Engine.PrimitiveComponent))
  (Variables|Default|SetProjectile%20Material _returnvalue)
  (Transformation|SetWorldScale3D (Variables|Default|GetStaticMesh) (Variables|Default|GetScale))
  (Variables|/Script/Engine.ProjectileMovementComponent|SetMaxSpeed _projectilemovement _speed)
  (Variables|/Script/Engine.ProjectileMovementComponent|SetInitialSpeed _projectilemovement _speed))